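; BP_OpenableDoor is a door actor that swings open and closed on requests from its OpenDoor component.
; It stores its starting rotation on BeginPlay, and the open and close events play or reverse the DoorMovement timeline.
; The timeline's OpenAngle track drives yaw relative to that starting rotation, and its event track plays the Doorlock sound at the door's location.
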(event `self.ReceiveBeginPlay`
  (set `self.InitialRotation` (`self.K2_GetActorRotation`)))

(event `self.OpenDoor.OnOpenRequest`
  (bind (_direction _open_angle) (`Timeline|DoorMovement` :!label _label)
    (:`Update`
      (`self.K2_SetActorRotation` (`KismetMathLibrary.ComposeRotators` (`KismetMathLibrary.MakeRotator` 0.0 0.0 _open_angle) (`self.InitialRotation`))))
    (:`Sound Event`
      (`GameplayStatics.PlaySoundAtLocation` "/Game/Audio/door-lock.door-lock" (`self.K2_GetActorLocation`) (struct) 1.0 1.0 0.0 null null null))))

(event `self.OpenDoor.OnCloseRequest`
  (goto _label :!via `Reverse`))

(fn `UserConstructionScript`)